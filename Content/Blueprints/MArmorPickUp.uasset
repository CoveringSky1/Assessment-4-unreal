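; MArmorPickUp is an armor pickup actor that comes in four rarities: Common, Rare, Master and Legendary.
; On BeginPlay it calls OnGenerate, then sets the skeletal mesh material to match its Rarity.
; When picked up, it looks for an Armor component on the collecting actor, sets that component's CurrentArmor to its Buff value and destroys itself.
; Actors without an Armor component leave the pickup in place.
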(event EventBeginPlay
  (Class|ArmorPickUp|OnGenerate)
  (switch Utilities|FlowControl|Switch|SwitchonEArmorPickupRarity (Variables|Default|GetRarity)
    (:LEGENDARY
      (Rendering|Material|SetMaterial (Variables|Default|GetSkeletalMesh) 0 "/Game/Materials/PickupMaterials/LegendaryMaterial.LegendaryMaterial"))
    (:MASTER
      (Rendering|Material|SetMaterial (Variables|Default|GetSkeletalMesh) 0 "/Game/Materials/PickupMaterials/MasterMaterial.MasterMaterial"))
    (:RARE
      (Rendering|Material|SetMaterial (Variables|Default|GetSkeletalMesh) 0 "/Game/Materials/PickupMaterials/RareMaterial.RareMaterial"))
    (:COMMON
      (Rendering|Material|SetMaterial (Variables|Default|GetSkeletalMesh) 0 "/Game/Materials/PickupMaterials/CommonMaterial.CommonMaterial"))))

(event Collision|EventActorBeginOverlap
  (params (OtherActor :type Actor%20Object%20Reference)))

(event EventTick
  (params (DeltaSeconds :type Float%20%28single-precision%29)))

(event EventOnPickup
  (params (ActorThatPickedUp :type Actor%20Object%20Reference))
  (bind _returnvalue (Actor|GetComponentbyClass ActorThatPickedUp "/Script/AdvGamesProgramming.Armor"))
  (Utilities|IsValid _returnvalue
    (:Is%20Valid
      (Variables|/Script/AdvGamesProgramming.Armor|SetCurrentArmor _returnvalue (Variables|Default|GetBuff))
      (Actor|DestroyActor))))

(fn ConstructionScript)