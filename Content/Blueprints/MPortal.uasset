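; MPortal is a pickup portal that clears the current map and triggers a new one once the coin manager's TotalGoldenCoin is zero.
; On pickup it checks GoldenCoinManage actors, then destroys all doors, PCG map actors, and coin, armor, health and weapon pickups.
; It then sets RegenerateMap on each MyPlaceNode and, inside that loop, zeroes the collector's GoldenCoin counts and flags a refresh.
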(event EventBeginPlay)

(event Collision|EventActorBeginOverlap
  (params (OtherActor :type Actor%20Object%20Reference)))

(event EventTick
  (params (DeltaSeconds :type Float%20%28single-precision%29)))

(event EventOnPickup
  (params (ActorThatPickedUp :type Actor%20Object%20Reference))
  (bind _returnvalue (Actor|GetComponentbyClass ActorThatPickedUp "/Game/Blueprints/GoldenCoin.GoldenCoin_C"))
  (bind _outactors (Actor|GetAllActorsOfClass "/Game/Blueprints/goldenCoinManage.goldenCoinManage_C"))
  (for _array_element _outactors
    (Utilities|IsValid "/Game/Blueprints/goldenCoinManage.goldenCoinManage"
      (:Is%20Valid
        (if (== (Variables|/Game/Blueprints/goldenCoinManage.goldenCoinManage_C|GetTotalGoldenCoin _array_element) 0)
          (Utilities|FlowControl|Sequence
            (:then_0
              (bind _outactors_2 (Actor|GetAllActorsOfClass "/Game/Blueprints/Door.Door_C"))
              (for _array_element_2 _outactors_2
                (Actor|DestroyActor _array_element_2)))
            (:then_1
              (bind _outactors_3 (Actor|GetAllActorsOfClass "/Game/Blueprints/Mypcgmap.Mypcgmap_C"))
              (for _array_element_3 _outactors_3
                (Actor|DestroyActor _array_element_3)))
            (:then_2
              (bind _outactors_4 (Actor|GetAllActorsOfClass "/Game/Blueprints/MGoldenCoinPickUp.MGoldenCoinPickUp_C"))
              (for _array_element_4 _outactors_4
                (Actor|DestroyActor _array_element_4)))
            (:then_3
              (bind _outactors_5 (Actor|GetAllActorsOfClass "/Game/Blueprints/MArmorPickUp.MArmorPickUp_C"))
              (for _array_element_5 _outactors_5
                (Actor|DestroyActor _array_element_5)))
            (:then_4
              (bind _outactors_6 (Actor|GetAllActorsOfClass "/Game/Blueprints/MyHealthPickUp.MyHealthPickUp_C"))
              (for _array_element_6 _outactors_6
                (Actor|DestroyActor _array_element_6)))
            (:then_5
              (bind _outactors_7 (Actor|GetAllActorsOfClass "/Game/Blueprints/WeaponPickupBlueprint.WeaponPickupBlueprint_C"))
              (for _array_element_7 _outactors_7
                (Actor|DestroyActor _array_element_7)))
            (:then_6
              (bind _outactors_8 (Actor|GetAllActorsOfClass "/Game/Blueprints/MyPlaceNode.MyPlaceNode_C"))
              (for _array_element_8 _outactors_8
                (Variables|/Script/AdvGamesProgramming.PlaceNode|SetbRegenerateMap _array_element_8 true)
                (Variables|/Game/Blueprints/GoldenCoin.GoldenCoin_C|SetCurrentGoldenCoin _returnvalue 0)
                (Variables|/Game/Blueprints/GoldenCoin.GoldenCoin_C|SetTotalGoldenCoin _returnvalue 0)
                (Variables|/Game/Blueprints/GoldenCoin.GoldenCoin_C|Setrefresh _returnvalue true)))))))))

(fn ConstructionScript)